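; Lockpicking component that runs a rotate-the-pin minigame on a locked object, with a random sweet-spot range narrowed by difficulty.
; Interacting toggles the player's WBP_Lockpick widget and blocks move and look input, while horizontal mouse movement rotates the pin.
; Tick eases the lock's turn while trying, capping it by the pin's angular error outside the range.
; A full 90-degree turn unlocks it and closes the minigame.
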(event `Initialize`
  (params (LockedState :type Boolean) (Difficulty :type "/Game/LockpickingSystem/Blueprints/EDifficulty Enum" :default "NewEnumerator0"))
  (bind _output_get (set `self.isLocked` LockedState))
  (if _output_get
    (bind _output_get_2 (set `self.PinRangeMin` (`KismetMathLibrary.RandomFloatInRange` 0.0 160.0)))
    (set `self.PinRangeMax` (+ _output_get_2 (select `/Game/LockpickingSystem/Blueprints/EDifficulty` Difficulty :`NewEnumerator0` 20.0 :`NewEnumerator4` 15.0 :`NewEnumerator2` 10.0 :`NewEnumerator3` 5.0 :!type "Float (single-precision)")))))

(event `self.ReceiveTick`
  (params (DeltaSeconds :type "Float (single-precision)"))
  (bind _pinangle (`self.GetPinAngle`))
  (bind _pinangle_2 (`self.GetPinAngle`))
  (bind _lockpickingtime (`self.LockpickingTime`))
  (bind _lockpickwidget (`self.LockpickWidget`))
  (bind _lockpickwidget_2 (`self.LockpickWidget`))
  (bind _returnvalue (`KismetMathLibrary.Abs` (- _pinangle_2 (`self.PinRangeMax`))))
  (bind _returnvalue_2 (`KismetMathLibrary.Abs` (- _pinangle_2 (`self.PinRangeMin`))))
  (`|ExecutionSequence`
    (:`then_0`
      ;[1 1 1] Freeze Rotate Pin in Trying Lockpick
      (`/Engine/EditorBlueprintResources/StandardMacros.IsValid` _lockpickwidget_2
        (:`Is Valid`
          (set `/Game/LockpickingSystem/UI/WBP_Lockpick.LockPin` (`self.TryingLockpick`) _lockpickwidget_2)
          (bind _output_get (set `self.LockpickingTime` (`KismetMathLibrary.FClamp` (`KismetMathLibrary.FInterpTo` (`self.LockpickingTime`) (select `bool` (`self.TryingLockpick`) :`false` -0.01 :`true` 1.1 :!type "Float (single-precision)") DeltaSeconds 3.0))))
          (bind _returnvalue_3 (`KismetMathLibrary.FClamp` (`|EaseFunction` "Linear" _output_get 0.0 90.0) 0.0 (- 90.0 (`KismetMathLibrary.FClamp` (* (select `bool` (and (>= _pinangle (`self.PinRangeMin`)) (<= _pinangle (`self.PinRangeMax`))) :`false` 1.0 :!type "Float (single-precision)") (select `bool` (< _returnvalue_2 _returnvalue) :`false` _returnvalue_2 :`true` _returnvalue)) 0.0 90.0))))
          (`Widget.SetRenderAngle` (`/Game/LockpickingSystem/UI/WBP_Lockpick.WBP_SmallLock` (`self.LockpickWidget`)) _returnvalue_3)
          (if (and (>= _returnvalue_3 90.0) (>= _lockpickingtime 1.0))
            (`/Engine/EditorBlueprintResources/StandardMacros.DoOnce` false
              (:`Completed`
                (set `self.isLocked` false)
                (`UserWidget.PlayAnimation` _lockpickwidget (`/Game/LockpickingSystem/UI/WBP_Lockpick.Fade_InOut` _lockpickwidget) 0.0 1 "Reverse" 1.0)
                (set `self.Lockpicking` false)
                (set `self.TryingLockpick` false)
                (`self.SetIgnoreMoveTurn` false)))
            (elif (>= _lockpickingtime 0.6666)
              (`/Engine/EditorBlueprintResources/StandardMacros.DoOnce` false :!label _label
                (:`Completed`
                  (`/Engine/EditorBlueprintResources/StandardMacros.IncrementInt` (`self.Counter`))))
              (else
                (goto _label :!via `Reset`)))))))
    (:`then_1`
      ;[1 1 1] Handle Pin Rotate
      (if (`self.Lockpicking`)
        (bind _returnvalue_4 (`WidgetLayoutLibrary.GetMousePositionOnViewport`))
        (`self.RotatePin` (- (`KismetMathLibrary.BreakVector2D` _returnvalue_4) (`self.X`)))
        (bind _returnvalue_5 (`WidgetLayoutLibrary.GetMousePositionOnViewport`))
        (set `self.X` (`KismetMathLibrary.BreakVector2D` _returnvalue_5))))))

(fn `DisplayRange`
  (params (Duration :type "Float (double-precision)"))
  (`KismetSystemLibrary.PrintString` (`KismetStringLibrary.Concat_StrStr` (`KismetSystemLibrary.GetDisplayName` (`self.GetOwner`)) " Range: (" (`KismetStringLibrary.Conv_DoubleToString` (`self.PinRangeMin`)) "," (`KismetStringLibrary.Conv_DoubleToString` (`self.PinRangeMax`)) ")") true true (struct :`G` 0.66 :`B` 1.0 :`A` 1.0) Duration))

(fn `GetLocpickWidget`
  (returns (Lockpick :type "/Game/LockpickingSystem/UI/WBP_Lockpick Object Reference"))
  (locals (WidgetLockpick :type "/Game/LockpickingSystem/UI/WBP_Lockpick Object Reference"))
  (bind _lockpickpawn (`self.LockpickPawn`))
  (`/Engine/EditorBlueprintResources/StandardMacros.IsValid` _lockpickpawn
    (:`Is Valid`
      (bind _foundwidgets (`WidgetBlueprintLibrary.GetAllWidgetsOfClass` "/Game/LockpickingSystem/UI/WBP_Lockpick.WBP_Lockpick_C"))
      (for _array_element _foundwidgets
        (if (== (`Widget.GetOwningPlayer` _array_element) (`Pawn.GetController` _lockpickpawn))
          (set `local.WidgetLockpick` _array_element)
          (break)))
      (return (`local.WidgetLockpick`)))
    (:`Is Not Valid`
      (return (`local.WidgetLockpick`)))))

(fn `InteractLockpick`
  (params (LockpickPawn :type "Pawn Object Reference") (Controller :type "Controller Object Reference"))
  (bind _lockpickwidget (`self.LockpickWidget`))
  (bind _lockpickwidget_2 (`self.LockpickWidget`))
  (if (`self.isLocked`)
    (`/Engine/EditorBlueprintResources/StandardMacros.IsValid` LockpickPawn
      (:`Is Valid`
        (set `self.LockpickPawn` LockpickPawn)
        (bind _lockpick (`self.GetLocpickWidget`))
        (bind _output_get (set `self.LockpickWidget` _lockpick))
        (`/Engine/EditorBlueprintResources/StandardMacros.IsValid` _output_get
          (:`Is Valid`
            (if (`self.Lockpicking`)
              (set `self.Lockpicking` false)
              (`UserWidget.PlayAnimation` _lockpickwidget (`/Game/LockpickingSystem/UI/WBP_Lockpick.Fade_InOut` _lockpickwidget) 0.0 1 "Reverse" 1.0)
              (`self.SetIgnoreMoveTurn` false)
              (elif (`self.isLocked`)
                (set `self.Lockpicking` true)
                (`UserWidget.PlayAnimation` _lockpickwidget_2 (`/Game/LockpickingSystem/UI/WBP_Lockpick.Fade_InOut` _lockpickwidget_2) 0.0 1 "Forward" 1.0)
                (`self.SetIgnoreMoveTurn` true)))))))))

(fn `RotatePin`
  (params (value :type "Float (double-precision)"))
  (bind _lockpickwidget (`self.LockpickWidget`))
  (if (and (>= (`KismetMathLibrary.Abs` value) 0.2) (not (`self.TryingLockpick`)) (`self.Lockpicking`))
    (`/Engine/EditorBlueprintResources/StandardMacros.IsValid` _lockpickwidget
      (:`Is Valid`
        (`/Game/LockpickingSystem/UI/WBP_Lockpick.RotatePin` _lockpickwidget value))
      (:`Is Not Valid`
        (`KismetSystemLibrary.PrintString` "Hello")))))

(fn `SetIgnoreMoveTurn`
  (params (isIgnore :type Boolean))
  (bind _lockpickpawn (`self.LockpickPawn`))
  (bind _returnvalue (`Pawn.GetController` _lockpickpawn))
  (`/Engine/EditorBlueprintResources/StandardMacros.IsValid` _lockpickpawn
    (:`Is Valid`
      (`Controller.SetIgnoreLookInput` _returnvalue isIgnore)
      (`Controller.SetIgnoreMoveInput` _returnvalue isIgnore))))

(fn `TryLockpicking`
  (params (isPressed :type Boolean))
  (if (and (`self.Lockpicking`) (`self.isLocked`))
    (set `self.TryingLockpick` isPressed)))