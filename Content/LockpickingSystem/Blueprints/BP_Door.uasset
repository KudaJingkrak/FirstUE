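; Lockable door actor that players open and close, or lockpick while it is locked.
; A box overlap enables input for the player and stores their pawn.
; Examine or Interact starts lockpicking through the lockpick component when locked and toggles the door otherwise, while Use press and release drive the picking attempt.
; Tick interpolates the mesh yaw between closed and open.
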(event `ToggleDoor`
  (if (not (`/Game/LockpickingSystem/Blueprints/LockpickCompoent.isLocked` (`self.LockpickCompoent`)))
    (set `self.isClosed` (not (`self.isClosed`)))))

(event `self.ReceiveBeginPlay`
  (bind _lockpickcompoent (`self.LockpickCompoent`))
  (`/Game/LockpickingSystem/Blueprints/LockpickCompoent.Initialize` _lockpickcompoent (`self.LockedState`) (`self.Difficulty`))
  (`/Game/LockpickingSystem/Blueprints/LockpickCompoent.DisplayRange` _lockpickcompoent 120.0))

(event `self.ReceiveTick`
  (params (DeltaSeconds :type "Float (single-precision)"))
  (bind _sm_door (`self.SM_Door`))
  (bind (_relativerotation_roll _relativerotation_pitch _relativerotation_yaw) (`KismetMathLibrary.BreakRotator` (`SceneComponent.RelativeRotation` _sm_door)))
  (`|ExecutionSequence`
    (:`then_0`
      ;[1 1 1] Handle toggle door
      (`SceneComponent.K2_SetRelativeRotation` _sm_door (`KismetMathLibrary.MakeRotator` 0.0 0.0 (`KismetMathLibrary.FInterpTo` _relativerotation_yaw (select `bool` (`self.isClosed`) :`false` 90.0 :!type "Float (single-precision)") DeltaSeconds (`self.DoorSpeed`))) false false))))

(event `InputAction|[HE]Use`
  (params (Key :type "Key Structure"))
  (bind _controlledpawn (`self.ControlledPawn`))
  (bind _lockpickcompoent (`self.LockpickCompoent`))
  (:`Pressed`
    (`/Engine/EditorBlueprintResources/StandardMacros.IsValid` _controlledpawn
      (:`Is Valid`
        (`/Game/LockpickingSystem/Blueprints/LockpickCompoent.TryLockpicking` _lockpickcompoent true))))
  (:`Released`
    (`/Engine/EditorBlueprintResources/StandardMacros.IsValid` _controlledpawn
      (:`Is Valid`
        (`/Game/LockpickingSystem/Blueprints/LockpickCompoent.TryLockpicking` _lockpickcompoent false)))))

(event `/Game/LockpickingSystem/Blueprints/BPI_Interaction.Interact`
  (params (InteractActor :type "Actor Object Reference"))
  (bind _controlledpawn (`self.ControlledPawn`))
  (bind _lockpickcompoent (`self.LockpickCompoent`))
  (`/Engine/EditorBlueprintResources/StandardMacros.IsValid` _controlledpawn :!label _label
    (:`Is Valid`
      (if (`/Game/LockpickingSystem/Blueprints/LockpickCompoent.isLocked` _lockpickcompoent)
        (`/Game/LockpickingSystem/Blueprints/LockpickCompoent.InteractLockpick` _lockpickcompoent _controlledpawn null)
        (else
          (`self.ToggleDoor`))))))

(event `InputAction|[HE]Examine`
  (params (Key :type "Key Structure"))
  (:`Pressed`
    (goto _label)))

(event `self.Box.OnComponentBeginOverlap`
  (params (OverlappedComponent :type "PrimitiveComponent Object Reference") (OtherActor :type "Actor Object Reference") (OtherComp :type "PrimitiveComponent Object Reference") (OtherBodyIndex :type Integer) (bFromSweep :type Boolean) (SweepResult :type "HitResult Structure (by ref)"))
  (bind _ascharacter (cast `Character` OtherActor))
  (bind _asplayer_controller (cast `PlayerController` (`Pawn.GetController` _ascharacter)))
  (`self.EnableInput` _asplayer_controller)
  (set `self.ControlledPawn` (`Controller.K2_GetPawn` _asplayer_controller)))

(event `self.Box.OnComponentEndOverlap`
  (params (OverlappedComponent :type "PrimitiveComponent Object Reference") (OtherActor :type "Actor Object Reference") (OtherComp :type "PrimitiveComponent Object Reference") (OtherBodyIndex :type Integer))
  (bind _ascharacter (cast `Character` OtherActor))
  (bind _asplayer_controller (cast `PlayerController` (`Pawn.GetController` _ascharacter)))
  (`self.DisableInput` _asplayer_controller))

(fn `UserConstructionScript`)