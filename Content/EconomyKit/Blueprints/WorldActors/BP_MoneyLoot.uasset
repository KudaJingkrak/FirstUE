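; BP_MoneyLoot is an Economy Kit world actor that represents a pile of money loot, sized by its MoneyToPickUp amount.
; SetupCoin swaps the static mesh between low, medium, heavy and ultra coin models using descending amount thresholds, falling back to the low model.
; It runs from both the construction script and BeginPlay.
; This Blueprint's graphs handle only the visual, with no pickup logic.
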(event `self.ReceiveBeginPlay`
  ;[1 1 1] Setup the coin
  (`self.SetupCoin`))

(fn `SetupCoin`
  (bind _moneytopickup (`self.MoneyToPickUp`))
  ;[1 1 1] Based on coin amount pick a differen mesh
  (`StaticMeshComponent.SetStaticMesh` (`self.StaticMesh`) (select `bool` (> _moneytopickup 9999) :`false` (select `bool` (> _moneytopickup 4999) :`false` (select `bool` (> _moneytopickup 1499) :`false` (select `bool` (> _moneytopickup -1) :`false` "/Game/EconomyKit/Meshes/Coins/SM_LowCoins.SM_LowCoins" :`true` "/Game/EconomyKit/Meshes/Coins/SM_LowCoins.SM_LowCoins" :!type "StaticMesh Object Reference") :`true` "/Game/EconomyKit/Meshes/Coins/SM_MediumCoins.SM_MediumCoins") :`true` "/Game/EconomyKit/Meshes/Coins/SM_HeavyCoins.SM_HeavyCoins") :`true` "/Game/EconomyKit/Meshes/Coins/SM_UltraCoins.SM_UltraCoins")))

(fn `UserConstructionScript`
  (`self.SetupCoin`))