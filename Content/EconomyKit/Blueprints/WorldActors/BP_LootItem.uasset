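; Replicated-world loot pickup actor that represents an item ID and amount lying in the world.
; SetupMesh, run at construction and BeginPlay, sets the mesh from the item's required info and clamps Amount to that item's max stack.
; An optional LockedBy controller reserves the item: CanBePickedUpBy admits only that controller, and the server clears the lock 60 seconds after BeginPlay.
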(event `self.ReceiveBeginPlay`
  ;[1 1 1] Setup the mesh and settings
  (`self.SetupMesh`)
  (`/Engine/EditorBlueprintResources/ActorMacros.Switch Has Authority`
    (:`Authority`
      (`/Engine/EditorBlueprintResources/StandardMacros.IsValid` (`self.LockedBy`)
        (:`Is Valid`
          (`KismetSystemLibrary.K2_SetTimerDelegate` (delegate `ClearOwned`) 60.0))))))

(event `ClearOwned`
  ;[1 1 1] Setup the mesh and settings
  (set `self.LockedBy` null))

(fn `CanBePickedUpBy`
  (params (InController :type "Actor Object Reference"))
  (returns (bCan :type Boolean))
  (bind _lockedby (`self.LockedBy`))
  (`/Engine/EditorBlueprintResources/StandardMacros.IsValid` _lockedby
    (:`Is Valid`
      (if (== InController _lockedby)
        (return true)
        (else
          (return false))))
    (:`Is Not Valid`
      (return true))))

(fn `SetupMesh`
  (bind (_friendlyname _bcanstack _maxstack _itemdescription _rarity _type _texture _buycost _sellcost _mesh) (`/Game/EconomyKit/Blueprints/Lib/EconomyHelpers.GetItemRequiredInfo` (`self.ID`)))
  ;[1 1 1] Set max stack and clamp the amount to max staxck
  (`StaticMeshComponent.SetStaticMesh` (`self.StaticMesh`) _mesh)
  (if (> (`self.Amount`) _maxstack)
    (set `self.Amount` _maxstack)))

(fn `UserConstructionScript`
  (`self.SetupMesh`))