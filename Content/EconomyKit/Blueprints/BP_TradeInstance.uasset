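; Replicated trade session actor that brokers an item and coin exchange between two players.
; Add and Remove shuffle items between each player's dummy inventory and replicated offer array, whose RepNotifies refresh both trading views.
; When both are ready, a multicast timestamps acceptance and timers set a lock flag, then finalize; un-readying cancels them.
; Finalizing rechecks readiness and elapsed time, applies real inventory and money changes, stops trading and expires the actor.
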(event `MC_AcceptBoth`
  ;[1 1 1] Multicast set both accept time
  (set `self.bBothAccepted` true)
  (set `self.BothAccepttime` (`KismetMathLibrary.UtcNow`)))

(fn `Add`
  (params (Player :type "/Game/EconomyKit/Blueprints/Enums/ETradePersn Enum") (ID :type String) (Amount :type Integer))
  (locals (PlayerIn :type "/Game/EconomyKit/Blueprints/Enums/ETradePersn Enum") (InString :type String) (InAmount :type Integer))
  (bind _playerin (`local.PlayerIn`))
  ;[1 1 1] Renove from dummy
  (if (`self.bFinished`)
    (return)
    (else
      (set `local.PlayerIn` Player)
      (set `local.InString` ID)
      (set `local.InAmount` Amount)
      (bind (_success _outinventory) (`/Game/EconomyKit/Blueprints/Lib/InventoryHelpers.RemoveFromInv` (`local.InAmount`) (`local.InString`) (select `/Game/EconomyKit/Blueprints/Enums/ETradePersn` (`local.PlayerIn`) :`NewEnumerator0` (`/Game/EconomyKit/Blueprints/BP_EconomyComp.DummyInventory` (`self.PlayerA`)) :`NewEnumerator1` (`/Game/EconomyKit/Blueprints/BP_EconomyComp.DummyInventory` (`self.PlayerB`)))))
      (if _success
        (set `/Game/EconomyKit/Blueprints/BP_EconomyComp.DummyInventory` _outinventory (select `/Game/EconomyKit/Blueprints/Enums/ETradePersn` (`local.PlayerIn`) :`NewEnumerator0` (`self.PlayerA`) :`NewEnumerator1` (`self.PlayerB`)))
        ;[1 1 1] Add to trade instance
        (bind _out (`/Game/EconomyKit/Blueprints/Lib/InventoryHelpers.AddTo` (select `/Game/EconomyKit/Blueprints/Enums/ETradePersn` _playerin :`NewEnumerator0` (`self.PlayerAArrray`) :`NewEnumerator1` (`self.PlayerBArray`)) (`local.InString`) (`local.InAmount`) (`self.PlayerA`)))
        (switch `/Game/EconomyKit/Blueprints/Enums/ETradePersn` _playerin
          (:`NewEnumerator0`
            (set `self.PlayerAArrray` _out))
          (:`NewEnumerator1`
            (set `self.PlayerBArray` _out)))
        (return)
        (else
          (return))))))

(fn `ChangeReady`
  (params (Player :type "/Game/EconomyKit/Blueprints/Enums/ETradePersn Enum") (bReady :type Boolean))
  ;[1 1 1] If not finished, set players ready and if both ready initiate countdown, if not cancel it if it exists
  (if (`self.bFinished`)
    (return)
    (else
      (switch `/Game/EconomyKit/Blueprints/Enums/ETradePersn` Player
        (:`NewEnumerator0`
          (set `self.bPlayer1Ready` bReady))
        (:`NewEnumerator1`
          (set `self.bPlayer2Ready` bReady)))
      (if (and (`self.bPlayer1Ready`) (`self.bPlayer2Ready`))
        (`self.MC_AcceptBoth`)
        (`KismetSystemLibrary.K2_SetTimer` null "Lock" (- (`self.ReadyTimeCheck`) 1.0))
        (`KismetSystemLibrary.K2_SetTimer` null "CheckFinalize" (+ (`self.ReadyTimeCheck`) 1.0))
        (return)
        (else
          (set `self.bBothAccepted` false)
          (`KismetSystemLibrary.K2_ClearTimer` null "Lock")
          (set `self.bLocked` false)
          (`KismetSystemLibrary.K2_ClearTimer` null "CheckFinalize")
          (return))))))

(fn `CheckFinalize`
  (bind _playerb (`self.PlayerB`))
  (bind _playera (`self.PlayerA`))
  ;[1 1 1] Not finished already?
  (if (`self.bFinished`)
    _
    (elif (and (and (`self.bPlayer1Ready`) (`self.bPlayer2Ready`)) (> (`.Seconds` (`KismetMathLibrary.BreakTimespan` (- (`KismetMathLibrary.UtcNow`) (`self.BothAccepttime`)))) (`KismetMathLibrary.FTrunc` (`self.ReadyTimeCheck`))))
      ;[1 1 1] Set finished to avoid any more changes
      (set `self.bFinished` true)
      ;[1 1 1] Remove from both their inventories and add to your inventories and give and substract money sent and given
      (for _array_element (`self.PlayerAArrray`)
        (bind (_id _amount) (break `/Game/EconomyKit/Blueprints/Structs/PlayerInventoryStruct` _array_element))
        (`/Game/EconomyKit/Blueprints/BP_EconomyComp.RemoveFromInventory` (`self.PlayerA`) _id _amount))
      (for _array_element_2 (`self.PlayerBArray`)
        (bind (_id_2 _amount_2) (break `/Game/EconomyKit/Blueprints/Structs/PlayerInventoryStruct` _array_element_2))
        (`/Game/EconomyKit/Blueprints/BP_EconomyComp.AddToInventory` (`self.PlayerA`) _id_2 _amount_2))
      (`/Game/EconomyKit/Blueprints/BP_EconomyComp.SubMoney` _playera (`self.Player1Coins`))
      (`/Game/EconomyKit/Blueprints/BP_EconomyComp.AddMoney` _playera (`self.Player2Coins`))
      (for _array_element_3 (`self.PlayerBArray`)
        (bind (_id_3 _amount_3) (break `/Game/EconomyKit/Blueprints/Structs/PlayerInventoryStruct` _array_element_3))
        (`/Game/EconomyKit/Blueprints/BP_EconomyComp.RemoveFromInventory` (`self.PlayerB`) _id_3 _amount_3))
      (for _array_element_4 (`self.PlayerAArrray`)
        (bind (_id_4 _amount_4) (break `/Game/EconomyKit/Blueprints/Structs/PlayerInventoryStruct` _array_element_4))
        (`/Game/EconomyKit/Blueprints/BP_EconomyComp.AddToInventory` (`self.PlayerB`) _id_4 _amount_4))
      (`/Game/EconomyKit/Blueprints/BP_EconomyComp.SubMoney` _playerb (`self.Player2Coins`))
      (`/Game/EconomyKit/Blueprints/BP_EconomyComp.AddMoney` _playerb (`self.Player1Coins`))
      (`/Game/EconomyKit/Blueprints/BP_EconomyComp.StopTrading` (`self.PlayerA`))
      (`/Game/EconomyKit/Blueprints/BP_EconomyComp.StopTrading` (`self.PlayerB`))
      (`self.SetLifeSpan` 1.5))))

(fn `Lock`
  ;[1 1 1] Make sure we're locked
  (set `self.bLocked` true)
  (return))

(fn `OnRep_PlayerAArrray`
  ;[1 1 1] Refresh
  (`/Game/EconomyKit/Blueprints/BP_EconomyComp.RefreshTrading` (`self.PlayerA`))
  (`/Game/EconomyKit/Blueprints/BP_EconomyComp.RefreshTrading` (`self.PlayerB`)))

(fn `OnRep_PlayerBArray`
  ;[1 1 1] Refresh
  (`/Game/EconomyKit/Blueprints/BP_EconomyComp.RefreshTrading` (`self.PlayerA`))
  (`/Game/EconomyKit/Blueprints/BP_EconomyComp.RefreshTrading` (`self.PlayerB`)))

(fn `Remove`
  (params (_PlayerIn :type "/Game/EconomyKit/Blueprints/Enums/ETradePersn Enum") (_InputPin :type String) (_InputPin1 :type Integer))
  (locals (PlayerIn :type "/Game/EconomyKit/Blueprints/Enums/ETradePersn Enum") (InString :type String) (InAmount :type Integer))
  (bind _returnvalue (select `/Game/EconomyKit/Blueprints/Enums/ETradePersn` (`local.PlayerIn`) :`NewEnumerator0` (`self.PlayerA`) :`NewEnumerator1` (`self.PlayerB`)))
  ;[1 1 1] If not finished remove add to the inventory and remove from the trade
  (if (`self.bFinished`)
    (return)
    (else
      (set `local.PlayerIn` _PlayerIn)
      (set `local.InString` _InputPin)
      (bind _output_get (set `local.InAmount` _InputPin1))
      (bind _out (`/Game/EconomyKit/Blueprints/Lib/InventoryHelpers.AddTo` (select `/Game/EconomyKit/Blueprints/Enums/ETradePersn` (`local.PlayerIn`) :`NewEnumerator0` (`/Game/EconomyKit/Blueprints/BP_EconomyComp.DummyInventory` (`self.PlayerA`)) :`NewEnumerator1` (`/Game/EconomyKit/Blueprints/BP_EconomyComp.DummyInventory` (`self.PlayerB`))) _InputPin _output_get _returnvalue))
      (set `/Game/EconomyKit/Blueprints/BP_EconomyComp.DummyInventory` _out _returnvalue)
      (bind (_success _outinventory) (`/Game/EconomyKit/Blueprints/Lib/InventoryHelpers.RemoveFromInv` _output_get _InputPin (select `/Game/EconomyKit/Blueprints/Enums/ETradePersn` (`local.PlayerIn`) :`NewEnumerator0` (`self.PlayerAArrray`) :`NewEnumerator1` (`self.PlayerBArray`))))
      (if _success
        (switch `/Game/EconomyKit/Blueprints/Enums/ETradePersn` (`local.PlayerIn`)
          (:`NewEnumerator0`
            (set `self.PlayerAArrray` _outinventory))
          (:`NewEnumerator1`
            (set `self.PlayerBArray` _outinventory)))
        (return)
        (else
          (return))))))

(fn `SetMoney`
  (params (Person :type "/Game/EconomyKit/Blueprints/Enums/ETradePersn Enum") (Amount :type Integer))
  ;[1 1 1] If not finished update the coinds
  (if (`self.bFinished`)
    (return)
    (else
      (switch `/Game/EconomyKit/Blueprints/Enums/ETradePersn` Person
        (:`NewEnumerator0`
          (set `self.Player1Coins` Amount))
        (:`NewEnumerator1`
          (set `self.Player2Coins` Amount)))
      (return))))

(fn `UserConstructionScript`)