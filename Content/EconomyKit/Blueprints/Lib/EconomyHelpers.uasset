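; Function library for the EconomyKit vendor and inventory economy, written as an adaptation point for other inventory systems.
; Helpers look up ItemData rows, map rarity to colors, split money into gold, silver and bronze, and total inventory worth.
; Buy and sell functions move money through server calls on the economy component and message its owner about items.
; Drop actions accept only vendor-inventory transfers, with Shift or Ctrl setting quantity.
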(fn `BuyFromVendor`
  (params (Owner :type "Object Object Reference") (ItemID :type String) (Amount :type Integer))
  (returns (ReturnValue :type Boolean))
  (bind _returnvalue (* (`.BuyCost` (`self.GetItemRequiredInfo` ItemID)) Amount))
  ;[1 1 1] Buy from the vendor using the owner, item ID and amount. This function can be adapted to more easily buy from a vendor using another inventory system
  (bind _asvendor_widget (cast `/Game/EconomyKit/Widgets/VendorWidget` Owner)
    (:`then`
      (bind _economyref (`/Game/EconomyKit/Widgets/VendorWidget.Economyref` _asvendor_widget))
      (bind _bhasenoughspace (message `/Game/EconomyKit/Blueprints/Lib/EconomyInterface.HasEnoughSpace` (`ActorComponent.GetOwner` _economyref) ItemID Amount))
      (if _bhasenoughspace
        (if (`/Game/EconomyKit/Blueprints/BP_EconomyComp.HasEnoughMoney` _economyref _returnvalue)
          (`/Game/EconomyKit/Blueprints/BP_EconomyComp.SERVER_SubMoney` _economyref _returnvalue)
          (message `/Game/EconomyKit/Blueprints/Lib/EconomyInterface.EconomyBought` (`ActorComponent.GetOwner` _economyref) ItemID Amount)
          (return true)
          (else
            _)))
      (return false))
    (:`CastFailed`
      (return false))))

(fn `ColorByRarity`
  (params (Rarity :type "/Game/EconomyKit/Blueprints/Enums/ItemRarity Enum"))
  (returns (Linear :type "LinearColor Structure") (Slate :type "SlateColor Structure"))
  (bind _returnvalue (select `/Game/EconomyKit/Blueprints/Enums/ItemRarity` Rarity :`NewEnumerator0` (make `SlateColor` (struct :`R` 0.365 :`G` 0.365 :`B` 0.365 :`A` 1.0)) :`NewEnumerator1` (make `SlateColor` (struct :`R` 0.85 :`G` 0.85 :`B` 0.85 :`A` 1.0)) :`NewEnumerator2` (make `SlateColor` (struct :`R` 1.0 :`G` 0.955806 :`B` 0.823223 :`A` 1.0)) :`NewEnumerator3` (make `SlateColor` (struct :`R` 0.67 :`G` 0.07705 :`B` 0.461018 :`A` 1.0)) :`NewEnumerator4` (make `SlateColor` (struct :`R` 0.88 :`G` 0.676379 :`B` 0.115036 :`A` 1.0)) :`NewEnumerator5` (make `SlateColor` (struct :`R` 1.0 :`G` 0.205652 :`A` 1.0)) :!type "SlateColor Structure"))
  ;[1 1 1] Depending on rarity, get a color
  (return (`.SpecifiedColor` (break `SlateColor` _returnvalue)) _returnvalue))

(fn `ConvertToCoinTypes`
  (params (Amount :type Integer))
  (returns (Gold :type Integer) (Silver :type Integer) (Bronze :type Integer))
  (bind _returnvalue (/ Amount 10000))
  (bind _returnvalue_2 (- Amount (* _returnvalue 10000)))
  (bind _returnvalue_3 (/ _returnvalue_2 100))
  ;[1 1 1] Calculate the coin types
  (return _returnvalue _returnvalue_3 (- _returnvalue_2 (* _returnvalue_3 100))))

(fn `CreateDropAction`
  (params (Object :type "Object Object Reference") (IsVendorItem :type Boolean))
  (returns (ReturnValue :type Boolean) (SellAmount :type Integer) (buyAmount :type Integer) (ItemID :type String) (Owner :type "UserWidget Object Reference") (bIsVendor :type Boolean))
  (locals (LocalOwner :type "UserWidget Object Reference") (LocalItem :type String) (bIsVendorItem :type Boolean) (bIsOwnerVendor :type Boolean))
  ;[1 1 1] When we drop get the griditem and values. Can be used to adapt to another inventory
  (set `local.bIsOwnerVendor` IsVendorItem)
  (bind _asgrid_item (cast `/Game/EconomyKit/Widgets/GridItem` Object)
    (:`then`
      (set `local.LocalOwner` (`/Game/EconomyKit/Widgets/GridItem.Owner` _asgrid_item))
      (set `local.LocalItem` (`/Game/EconomyKit/Widgets/GridItem.ID` _asgrid_item))
      (bind _bvendoritem (`/Game/EconomyKit/Widgets/GridItem.bVendorItem` _asgrid_item))
      (set `local.bIsVendorItem` _bvendoritem)
      (if (!= (`local.bIsOwnerVendor`) _bvendoritem)
        (bind (_buy _sell) (`self.DetermineAmount` (`/Game/EconomyKit/Widgets/GridItem.Amount` _asgrid_item)))
        (return true _sell _buy (`local.LocalItem`) (`local.LocalOwner`) (`local.bIsVendorItem`))
        (else
          (return false 0 0 "" null false))))
    (:`CastFailed`
      (return false 0 0 "" null false))))

(fn `DetermineAmount`
  (params (Amount :type Integer))
  (returns (Buy :type Integer) (Sell :type Integer))
  (bind _returnvalue (`GameplayStatics.GetPlayerController` null))
  (bind _returnvalue_2 (`PlayerController.IsInputKeyDown` _returnvalue "LeftControl"))
  (bind _returnvalue_3 (select `bool` (`PlayerController.IsInputKeyDown` _returnvalue "LeftShift") :`false` 1 :`true` 5))
  ;[1 1 1] If shift or ctrl down, if so use 5 or 10 as amount
  (return (select `bool` _returnvalue_2 :`false` _returnvalue_3 :`true` 10) (select `bool` _returnvalue_2 :`false` _returnvalue_3 :`true` Amount)))

(fn `GetItemRequiredInfo`
  (params (ID :type String))
  (returns (FriendlyName :type String) (bCanStack :type Boolean) (MaxStack :type Integer) (ItemDescription :type String) (Rarity :type "/Game/EconomyKit/Blueprints/Enums/ItemRarity Enum") (Type :type "/Game/EconomyKit/Blueprints/Enums/ItemType Enum") (Texture :type "Texture2D Object Reference") (BuyCost :type Integer) (SellCost :type Integer) (Mesh :type "StaticMesh Object Reference"))
  ;[1 1 1] This function can potententially be used to integrate another inventory with
  (bind _returnvalue (`|GetDataTableRow` "/Game/EconomyKit/Blueprints/Data/ItemData.ItemData" (`KismetStringLibrary.Conv_StringToName` ID))
    (:`then`
      (bind (_id _friendlyname _bcanstack _maxstack _itemdescription _rarity _type _texture _buycost _sellcost _mesh) (break `/Game/EconomyKit/Blueprints/Structs/ItemDataStruct` _returnvalue))
      (return _friendlyname _bcanstack _maxstack _itemdescription (cast `/Game/EconomyKit/Blueprints/Enums/ItemRarity` _rarity) (cast `/Game/EconomyKit/Blueprints/Enums/ItemType` _type) _texture _buycost _sellcost _mesh))
    (:`RowNotFound`
      (return "" false 0 "" "NewEnumerator0" "NewEnumerator0" null 0 0 null))))

(fn `InventoryWorth`
  (params (Inventory :type "Array of /Game/EconomyKit/Blueprints/Structs/PlayerInventoryStruct Structure"))
  (returns (CollectivePrice :type Integer))
  (locals (Collective :type Integer))
  ;[1 1 1] Worth of the inventory
  (for _array_element Inventory
    (bind (_id _amount) (break `/Game/EconomyKit/Blueprints/Structs/PlayerInventoryStruct` _array_element))
    (set `local.Collective` (+ (* _amount (`/Game/EconomyKit/Blueprints/Lib/InventoryHelpers.GetItemSellPrice` _id)) (`local.Collective`))))
  (return (`local.Collective`)))

(fn `SellFromInventory`
  (params (Owner :type "UserWidget Object Reference") (ItemID :type String) (ItemAmount :type Integer))
  (returns (ReturnValue :type Boolean))
  (locals (Amount :type Integer) (ID :type String) (LocalOwner :type "UserWidget Object Reference"))
  ;[1 1 1] Sell from the inventory, can be used to more easily use other inventory systems
  (set `local.ID` ItemID)
  (set `local.LocalOwner` Owner)
  (set `local.Amount` ItemAmount)
  (bind _asinventory_widget (cast `/Game/EconomyKit/Widgets/InventoryWidget` (`local.LocalOwner`))
    (:`then`
      (bind _economycomp (`/Game/EconomyKit/Widgets/InventoryWidget.EconomyComp` _asinventory_widget))
      (bind _returnvalue (`KismetMathLibrary.Clamp` (`local.Amount`) 1 (`/Game/EconomyKit/Blueprints/BP_EconomyComp.OwnsAmountOfID` _economycomp (`local.ID`))))
      (`/Game/EconomyKit/Blueprints/BP_EconomyComp.SERVER_AddMoney` _economycomp (* (`.SellCost` (`self.GetItemRequiredInfo` (`local.ID`))) _returnvalue))
      (message `/Game/EconomyKit/Blueprints/Lib/EconomyInterface.EconomySell` (`ActorComponent.GetOwner` _economycomp) (`local.ID`) _returnvalue)
      (return true))
    (:`CastFailed`
      (return false))))