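; Inventory helper library for the economy kit that adds and removes items in stack-based inventory arrays and looks up item data.
; AddTo tops up the first non-full stack, then appends MaxStack-capped stacks, using stack rules from the passed-in Economy object.
; RemoveFromInv drains matching stacks in array order, returning a success flag and the resulting array.
; Removal-side lookups and sell prices read the ItemData table directly, with -1 marking missing prices.
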(fn `AddTo`
  (params (In :type "Array of /Game/EconomyKit/Blueprints/Structs/PlayerInventoryStruct Structure") (ToAddId1 :type String) (InputPin :type Integer) (Economy :type "/Game/EconomyKit/Blueprints/BP_EconomyComp Object Reference"))
  (returns (Out :type "Array of /Game/EconomyKit/Blueprints/Structs/PlayerInventoryStruct Structure"))
  (locals (ToAddId :type String) (ToAdd :type Integer) (InventoryStruct :type "Array of /Game/EconomyKit/Blueprints/Structs/PlayerInventoryStruct Structure") (Economyt :type "/Game/EconomyKit/Blueprints/BP_EconomyComp Object Reference") (RememberAdd :type Integer))
  (bind _toadd (`local.ToAdd`))
  (bind _inventorystruct (`local.InventoryStruct`))
  (bind _toaddid (`local.ToAddId`))
  (bind _toaddid_2 (`local.ToAddId`))
  (bind _maxstack (`/Game/EconomyKit/Blueprints/BP_EconomyComp.FindItemIdInfo` (`local.Economyt`) _toaddid_2))
  (bind (_bfound _stackamount _bstackable _lefttoadd _idout) (`self.FindnInvItem` (`local.InventoryStruct`) _toaddid (`local.Economyt`)))
  (bind (_bfound_2 _stackamount_2 _bstackable_2 _lefttoadd_2 _idout_2) (`self.FindnInvItem` (`local.InventoryStruct`) _toaddid_2 (`local.Economyt`)))
  (bind _maxstack_2 (`/Game/EconomyKit/Blueprints/BP_EconomyComp.FindItemIdInfo` (`local.Economyt`) _toaddid))
  (bind _returnvalue (+ (`local.ToAdd`) (`.Amount_5_F0D62B42432AF5958E3F25994B68E3FB` (break `/Game/EconomyKit/Blueprints/Structs/PlayerInventoryStruct` (`KismetArrayLibrary.Array_Get` (`local.InventoryStruct`) _idout)))))
  ;[1 1 1] Set the local variables, if client pass to server
  (set `local.ToAddId` ToAddId1)
  (bind _output_get (set `local.ToAdd` InputPin))
  (set `local.InventoryStruct` In)
  (set `local.Economyt` Economy)
  (if (<= _output_get 0)
    ;[1 1 1] If to add is 0 or less than 0 something is greatly wrong.
    (`KismetSystemLibrary.PrintString` null "ERROR: You tried to add something to the inventory with 0 or less than 0 amount. " true true (struct :`R` 1.0 :`A` 1.0) 8.0)
    (return (`local.InventoryStruct`))
    (else
      ;[1 1 1] Should we add to non-full exisiting stakcs or create new stacks?
      (if _bfound
        ;[1 1 1] Loop add to existing, non full stacks
        (if (> _lefttoadd 0)
          (if (> _returnvalue _maxstack)
            (set `local.RememberAdd` _lefttoadd_2)
            (`KismetArrayLibrary.Array_Set` _inventorystruct _idout_2 (make `/Game/EconomyKit/Blueprints/Structs/PlayerInventoryStruct` (`local.ToAddId`) _maxstack))
            (bind _output_get_2 (set `local.ToAdd` (- (`local.ToAdd`) (`local.RememberAdd`))))
            (`KismetSystemLibrary.PrintString` null (`KismetStringLibrary.Conv_IntToString` _output_get_2))
            (else
              (`KismetArrayLibrary.Array_Set` _inventorystruct _idout_2 (make `/Game/EconomyKit/Blueprints/Structs/PlayerInventoryStruct` (`local.ToAddId`) _returnvalue))
              (set `local.ToAdd` 0)))
          (if (> (`local.ToAdd`) 0)
            _
            (else
              ;[1 1 1] Update the inv UI
              (return (`local.InventoryStruct`))))))
      ;[1 1 1] Add new items until LeftToAdd is 0
      (if (<= _maxstack_2 (`local.ToAdd`)) :!label _label
        (`KismetArrayLibrary.Array_Add` (`local.InventoryStruct`) (make `/Game/EconomyKit/Blueprints/Structs/PlayerInventoryStruct` (`local.ToAddId`) _maxstack_2))
        (set `local.ToAdd` (- _toadd _maxstack_2))
        (else
          (`KismetArrayLibrary.Array_Add` (`local.InventoryStruct`) (make `/Game/EconomyKit/Blueprints/Structs/PlayerInventoryStruct` (`local.ToAddId`) _toadd))
          (set `local.ToAdd` 0)))
      (if (> (`local.ToAdd`) 0)
        (goto _label)
        (else
          (bind _output_get_3 (set `local.InventoryStruct` (`local.InventoryStruct`)))
          (return _output_get_3))))))

(fn `FindInvRemove`
  (params (Array :type "Array of /Game/EconomyKit/Blueprints/Structs/PlayerInventoryStruct Structure") (InputPin :type String))
  (returns (bFound :type Boolean) (StackAmount :type Integer) (bStackable :type Boolean) (LeftToAdd :type Integer) (IDOut :type Integer))
  (locals (LocalID :type Integer) (InventoryStruct :type "Array of /Game/EconomyKit/Blueprints/Structs/PlayerInventoryStruct Structure"))
  (bind (_return _maxstack) (`self.FindItemInfo` InputPin))
  (bind _localid (`local.LocalID`))
  (bind _localid_2 (`local.LocalID`))
  (bind (_id _amount) (break `/Game/EconomyKit/Blueprints/Structs/PlayerInventoryStruct` (`KismetArrayLibrary.Array_Get` (`local.InventoryStruct`) _localid)))
  (bind _output_get (set `local.InventoryStruct` Array))
  (for (_array_element _array_index) _output_get
    (if (`KismetStringLibrary.EqualEqual_StrStr` (`.Id_2_970A237D40F4B1D7EC551C95AC46623F` (break `/Game/EconomyKit/Blueprints/Structs/PlayerInventoryStruct` _array_element)) InputPin)
      (set `local.LocalID` _array_index)
      (break)))
  (if (> _localid -1)
    (return true _amount _return (select `bool` false :`true` (- _maxstack _amount)) _localid_2)
    (else
      (return false 0 _return 0 _localid_2))))

(fn `FindItemInfo`
  (params (InString :type String))
  (returns (Return :type Boolean) (MaxStack :type Integer))
  (bind _returnvalue (`|GetDataTableRow` "/Game/EconomyKit/Blueprints/Data/ItemData.ItemData" (`KismetStringLibrary.Conv_StringToName` InString))
    (:`then`
      (bind (_id _friendlyname _bcanstack _maxstack) (break `/Game/EconomyKit/Blueprints/Structs/ItemDataStruct` _returnvalue))
      (return _bcanstack _maxstack))
    (:`RowNotFound`
      (return false -1))))

(fn `FindnInvItem`
  (params (Array :type "Array of /Game/EconomyKit/Blueprints/Structs/PlayerInventoryStruct Structure") (InputPin :type String) (Inventory :type "/Game/EconomyKit/Blueprints/BP_EconomyComp Object Reference"))
  (returns (bFound :type Boolean) (StackAmount :type Integer) (bStackable :type Boolean) (LeftToAdd :type Integer) (IDOut :type Integer))
  (locals (InventoryStruct :type "Array of /Game/EconomyKit/Blueprints/Structs/PlayerInventoryStruct Structure") (LocalID :type Integer :default -1))
  (bind (_maxstack _bcanstack) (`/Game/EconomyKit/Blueprints/BP_EconomyComp.FindItemIdInfo` Inventory InputPin))
  (bind (_maxstack_2 _bcanstack_2) (`/Game/EconomyKit/Blueprints/BP_EconomyComp.FindItemIdInfo` Inventory InputPin))
  (bind _localid (`local.LocalID`))
  (bind _localid_2 (`local.LocalID`))
  (bind (_id _amount) (break `/Game/EconomyKit/Blueprints/Structs/PlayerInventoryStruct` (`KismetArrayLibrary.Array_Get` (`local.InventoryStruct`) _localid)))
  ;[1 1 1] Find item ID in inventory, if found we will see if it's stackable and how much more we can add to the stack
  (bind _output_get (set `local.InventoryStruct` Array))
  (for (_array_element _array_index) _output_get
    (bind (_id_2 _amount_2) (break `/Game/EconomyKit/Blueprints/Structs/PlayerInventoryStruct` _array_element))
    (if (`KismetStringLibrary.EqualEqual_StrStr` _id_2 InputPin)
      (if _bcanstack_2
        (if (< _amount_2 _maxstack_2)
          (set `local.LocalID` _array_index)
          (break)))))
  (if (> _localid -1)
    (return true _amount _bcanstack (select `bool` _bcanstack :`true` (- _maxstack _amount)) _localid_2)
    (else
      (return false 0 _bcanstack 0 _localid_2))))

(fn `GetItemSellPrice`
  (params (InString :type String))
  (returns (cost :type Integer))
  ;[1 1 1] Get sell price
  (bind _returnvalue (`|GetDataTableRow` "/Game/EconomyKit/Blueprints/Data/ItemData.ItemData" (`KismetStringLibrary.Conv_StringToName` InString))
    (:`then`
      (return (`.SellCost_28_1DBEF9F74B604A87D535D9AAB6043F6B` (break `/Game/EconomyKit/Blueprints/Structs/ItemDataStruct` _returnvalue))))
    (:`RowNotFound`
      (return -1))))

(fn `RemoveFromInv`
  (params (_ToRemove :type Integer) (_ToRemoveString :type String) (InInventory :type "Array of /Game/EconomyKit/Blueprints/Structs/PlayerInventoryStruct Structure"))
  (returns (Success :type Boolean) (OutInventory :type "Array of /Game/EconomyKit/Blueprints/Structs/PlayerInventoryStruct Structure"))
  (locals (ToRemove :type Integer) (ToRemoveString :type String) (InventoryStruct :type "Array of /Game/EconomyKit/Blueprints/Structs/PlayerInventoryStruct Structure"))
  ;[1 1 1] Set local vars, if client pass to server
  (if (<= _ToRemove 0)
    (`KismetSystemLibrary.PrintString` null "ERROR: Remove is amount 0")
    (return false (`local.InventoryStruct`))
    (else
      (set `local.ToRemove` _ToRemove)
      (bind _output_get (set `local.ToRemoveString` _ToRemoveString))
      (bind _output_get_2 (set `local.InventoryStruct` InInventory))
      (bind (_bfound _stackamount _bstackable _lefttoadd _idout) (`self.FindInvRemove` _output_get_2 _output_get))
      ;[1 1 1] Find the item to remove, if not found we return false
      (if _bfound
        ;[1 1 1] Remove from the inventory, if to remove  is smaller than stack amount let's adjust the stack, otherwise remove it and keep going until left to remove is 0
        (if (<= _stackamount (`local.ToRemove`)) :!label _label
          (if (<= (`KismetArrayLibrary.Array_Length` (`local.InventoryStruct`)) 0) :!label _label_2
            _
            (else
              (set `local.ToRemove` (- (`local.ToRemove`) _stackamount))
              (`KismetArrayLibrary.Array_Remove` (`local.InventoryStruct`) _idout)
              (if (> (`local.ToRemove`) 0)
                (goto _label)
                (else
                  (return true (`local.InventoryStruct`))))))
          (else
            (bind (_id _amount) (break `/Game/EconomyKit/Blueprints/Structs/PlayerInventoryStruct` (`KismetArrayLibrary.Array_Get` (`local.InventoryStruct`) _idout)))
            (bind _returnvalue (- _amount (`local.ToRemove`)))
            (if (< _returnvalue 0)
              (goto _label_2)
              (else
                (`KismetArrayLibrary.Array_Set` (`local.InventoryStruct`) _idout (make `/Game/EconomyKit/Blueprints/Structs/PlayerInventoryStruct` _id _returnvalue))))))
        (return true (`local.InventoryStruct`))
        (else
          (return false (`local.InventoryStruct`)))))))