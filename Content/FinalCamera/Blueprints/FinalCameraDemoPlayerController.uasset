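; Demo player controller that forwards movement, mouse, zoom and selection input to a FinalCameraManager.
; Keys switch TopDown, Shoulder, FirstPerson and FirstPersonArms presets with matching pawn rotation; zoom also crosses between shoulder and first person.
; Clicking retargets the camera to the hit actor, or locks its position at a BP_StaticCameraPosition.
; For FirstPersonArms, Tick waits until the camera is close, then hides the body and swaps in arms on a timer.
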(event `InputAction|EnableDisableScrollingMode`
  (params (Key :type "Key Structure" :default "AnyKey"))
  ;[1 0.3386 0.06699] Forward input to the camera
  ;;[1 1 1] Switches Scrolling mode on and off
  (:`Pressed`
    (`/Game/FinalCamera/Blueprints/FinalCameraManager.SwitchScrollingModeOnOff` (cast `/Game/FinalCamera/Blueprints/FinalCameraManager` (`self.PlayerCameraManager`) :!pure true))))

(event `InputAction|ZoomIn`
  (params (Key :type "Key Structure" :default "AnyKey"))
  (bind _returnvalue (`self.K2_GetPawn`))
  (bind _asfinal_camera_manager (cast `/Game/FinalCamera/Blueprints/FinalCameraManager` (`self.PlayerCameraManager`) :!pure true))
  ;[1 0.3386 0.06699] Forward input to the camera
  ;;[1 1 1] ZoomIn and ZoomOut; i guess this explains itself?
  (:`Pressed`
    (`/Game/FinalCamera/Blueprints/FinalCameraManager.ZoomInEvent` (cast `/Game/FinalCamera/Blueprints/FinalCameraManager` (`self.PlayerCameraManager`) :!pure true))
    ;[0.03393 0.1331 1] Zooming in from shouldercam to first person directly
    (if (and (== (`self.CurrentCameraMode`) "shoulder") (`KismetMathLibrary.NearlyEqual_FloatFloat` (`/Game/FinalCamera/Blueprints/FinalCameraManager.targetCamDistance` _asfinal_camera_manager) (`/Game/FinalCamera/Blueprints/FinalCameraManager.minCamDistance` _asfinal_camera_manager) 0.001))
      (`/Game/FinalCamera/Blueprints/FinalCameraManager.SetPresetCameraMode` _asfinal_camera_manager "FirstPerson" true)
      (set `self.CurrentCameraMode` "FirstPerson")
      (set `Pawn.bUseControllerRotationYaw` true _returnvalue)
      (set `Pawn.bUseControllerRotationPitch` true _returnvalue))))

(event `InputAxis|MoveForward`
  (params (AxisValue :type "Float (single-precision)"))
  (bind _returnvalue (`self.K2_GetPawn`))
  ;[1 0 0.4285] Character Movement handling
  ;;[1 1 1] Movement and turning around
  (if (!= AxisValue 0.0)
    (`Pawn.AddMovementInput` _returnvalue (`self.GetActorForwardVector` _returnvalue) AxisValue false)
    ;[1 1 1] When in ShoulderCam Mode, we want to let the player look around freely and only smoothly snap back behind the player when he is actually moving / turning
    (`/Game/FinalCamera/Blueprints/FinalCameraManager.FreeCamModeEventOff` (cast `/Game/FinalCamera/Blueprints/FinalCameraManager` (`self.PlayerCameraManager`) :!pure true) :!label _label)))

(event `InputAction|ZoomOut`
  (params (Key :type "Key Structure" :default "AnyKey"))
  (bind _returnvalue (`self.K2_GetPawn`))
  (bind _asfinal_camera_manager (cast `/Game/FinalCamera/Blueprints/FinalCameraManager` (`self.PlayerCameraManager`) :!pure true))
  ;[1 0.3386 0.06699] Forward input to the camera
  ;;[1 1 1] ZoomIn and ZoomOut; i guess this explains itself?
  (:`Pressed`
    (`/Game/FinalCamera/Blueprints/FinalCameraManager.ZoomOutEvent` (cast `/Game/FinalCamera/Blueprints/FinalCameraManager` (`self.PlayerCameraManager`) :!pure true))
    ;[0.03393 0.1331 1] Zooming in from shouldercam to first person directly
    (if (== (`self.CurrentCameraMode`) "FirstPerson")
      (`/Game/FinalCamera/Blueprints/FinalCameraManager.SetPresetCameraMode` _asfinal_camera_manager "Shoulder" true)
      (set `/Game/FinalCamera/Blueprints/FinalCameraManager.targetCamDistance` (`/Game/FinalCamera/Blueprints/FinalCameraManager.minCamDistance` _asfinal_camera_manager) _asfinal_camera_manager)
      (set `self.CurrentCameraMode` "shoulder")
      (set `Pawn.bUseControllerRotationYaw` true _returnvalue)
      (set `Pawn.bUseControllerRotationPitch` false _returnvalue)
      (`self.ResetPitch`))))

(event `InputAction|FreeLook`
  (params (Key :type "Key Structure" :default "AnyKey"))
  (bind _asfinal_camera_manager (cast `/Game/FinalCamera/Blueprints/FinalCameraManager` (`self.PlayerCameraManager`) :!pure true))
  ;[1 0.3386 0.06699] Forward input to the camera
  (:`Pressed`
    (set `self.bShowMouseCursor` false)
    (`/Game/FinalCamera/Blueprints/FinalCameraManager.FreeCamModeEventOn` _asfinal_camera_manager) ; FreeCamMode On means, no snapback to any original location
  )
  (:`Released`
    (set `self.bShowMouseCursor` true)
    ;[1 1 1] When in ShoulderCam Mode, we want to let the player look around freely and only smoothly snap back behind the player when he is actually moving / turning
    (if (!= (`self.CurrentCameraMode`) "shoulder")
      (`/Game/FinalCamera/Blueprints/FinalCameraManager.FreeCamModeEventOff` _asfinal_camera_manager))))

(event `InputAxis|TurnLeft`
  (params (AxisValue :type "Float (single-precision)"))
  ;[1 0 0.4285] Character Movement handling
  ;;[1 1 1] Movement and turning around
  (if (!= AxisValue 0.0)
    (`Pawn.AddControllerYawInput` (`self.K2_GetPawn`) AxisValue) ; Turn the character around
    (goto _label)))

(event `InputAxis|aMouseX` :consume false
  (params (AxisValue :type "Float (single-precision)"))
  ;[1 0.3386 0.06699] Forward input to the camera
  ;;[1 1 1] Forward mouse axis values to the CameraManager
  (`/Game/FinalCamera/Blueprints/FinalCameraManager.RawMouseEvent` (cast `/Game/FinalCamera/Blueprints/FinalCameraManager` (`self.PlayerCameraManager`) :!pure true) AxisValue (stale `InputAxis|aMouseY` AxisValue) :!label _label_2))

(event `InputAxis|aMouseX` :consume false
  (params (AxisValue :type "Float (single-precision)"))
  ;[1 0 0.4285] Character Movement handling
  ;;[1 1 1] Yaw and pitch input. Needed i.e. in first-person-mode
  (if (not (`/Game/FinalCamera/Blueprints/FinalCameraManager.isFreeCamMode` (cast `/Game/FinalCamera/Blueprints/FinalCameraManager` (`self.PlayerCameraManager`) :!pure true)))
    (`Pawn.AddControllerYawInput` (`self.K2_GetPawn`) AxisValue)))

(event `InputAction|ReAttach Camera`
  (params (Key :type "Key Structure" :default "AnyKey"))
  ;[0.05798 0.8561 1] Reset Camera Target to be our own Player Pawn again
  (:`Released`
    (`/Game/FinalCamera/Blueprints/FinalCameraManager.SetTargetActor` (cast `/Game/FinalCamera/Blueprints/FinalCameraManager` (`self.PlayerCameraManager`) :!pure true) (`self.K2_GetPawn`))))

(event `InputAxis|aMouseY` :consume false
  (params (AxisValue :type "Float (single-precision)"))
  ;[1 0.3386 0.06699] Forward input to the camera
  ;;[1 1 1] Forward mouse axis values to the CameraManager
  (goto _label_2))

(event `InputAxis|aMouseY` :consume false
  (params (AxisValue :type "Float (single-precision)"))
  ;[1 0 0.4285] Character Movement handling
  ;;[1 1 1] Yaw and pitch input. Needed i.e. in first-person-mode
  (if (not (`/Game/FinalCamera/Blueprints/FinalCameraManager.isFreeCamMode` (cast `/Game/FinalCamera/Blueprints/FinalCameraManager` (`self.PlayerCameraManager`) :!pure true)))
    (`Pawn.AddControllerPitchInput` (`self.K2_GetPawn`) (- AxisValue (* AxisValue 2.0)))))

(event `InputAction|DeSelect`
  (params (Key :type "Key Structure" :default "AnyKey"))
  (bind _asfinal_camera_manager (cast `/Game/FinalCamera/Blueprints/FinalCameraManager` (`self.PlayerCameraManager`) :!pure true))
  ;[0 0.7638 1] Reset our current Camera Target
  (:`Pressed`
    (`/Game/FinalCamera/Blueprints/FinalCameraManager.SetTargetActor` _asfinal_camera_manager null)
    (set `/Game/FinalCamera/Blueprints/FinalCameraManager.lockPosition` false _asfinal_camera_manager)))

(event `InputAction|Select`
  (params (Key :type "Key Structure" :default "AnyKey"))
  (bind (_bblockinghit _binitialoverlap _time _location _impactpoint _normal _impactnormal _physmat _hitactor) (`GameplayStatics.BreakHitResult` (`self.GetHitResultUnderCursorByChannel` "TraceTypeQuery2" true)))
  (bind _asfinal_camera_manager (cast `/Game/FinalCamera/Blueprints/FinalCameraManager` (`self.PlayerCameraManager`) :!pure true))
  ;[0 0.7638 1] If we clicked anywhere, set our new cameratarget to the actor we clicked on
  (:`Pressed`
    (if _bblockinghit
      (`/Engine/EditorBlueprintResources/StandardMacros.IsValid` _hitactor
        (:`Is Valid`
          (bind _asbp_static_camera_position (cast `/Game/FinalCamera/Blueprints/HelperBlueprints/BP_StaticCameraPosition` _hitactor)
            (:`then`
              ;;[1 0.8781 0.0519] If we are here it means that we clicked on a StaticCameraPosition Actor. This serves as a static camera point which cannot change its location but just the rotation, and stays focused on the targetactor
              (set `/Game/FinalCamera/Blueprints/FinalCameraManager.lockedPosition` (`self.K2_GetActorLocation` _asbp_static_camera_position) _asfinal_camera_manager)
              (set `/Game/FinalCamera/Blueprints/FinalCameraManager.lockPosition` true _asfinal_camera_manager))
            (:`CastFailed`
              (`/Game/FinalCamera/Blueprints/FinalCameraManager.SetTargetActor` (cast `/Game/FinalCamera/Blueprints/FinalCameraManager` (`self.PlayerCameraManager`) :!pure true) _hitactor))))))))

(event `Key|SpaceBar`
  (params (Key :type "Key Structure" :default "AnyKey"))
  (bind _returnvalue (`self.K2_GetPawn`))
  ;[0.065 1 0.1309] Setting different presets on the camera. If a preset has not been found, nothing is changed (view stays as is)
  (:`Pressed`
    (`self.ResetPitch`)
    (`/Game/FinalCamera/Blueprints/FinalCameraManager.SetPresetCameraMode` (cast `/Game/FinalCamera/Blueprints/FinalCameraManager` (`self.PlayerCameraManager`) :!pure true) "TopDown" true)
    (set `self.CurrentCameraMode` "TopDown")
    (set `Pawn.bUseControllerRotationYaw` true _returnvalue)
    (set `Pawn.bUseControllerRotationPitch` false _returnvalue)
    (`self.CheckAndSetMesh`)))

(event `Key|LeftAlt`
  (params (Key :type "Key Structure" :default "AnyKey"))
  (bind _returnvalue (`self.K2_GetPawn`))
  ;[0.065 1 0.1309] Setting different presets on the camera. If a preset has not been found, nothing is changed (view stays as is)
  (:`Pressed`
    (`self.ResetPitch`)
    (`/Game/FinalCamera/Blueprints/FinalCameraManager.SetPresetCameraMode` (cast `/Game/FinalCamera/Blueprints/FinalCameraManager` (`self.PlayerCameraManager`) :!pure true) "Shoulder" true)
    (set `self.CurrentCameraMode` "Shoulder")
    (set `Pawn.bUseControllerRotationYaw` true _returnvalue)
    (set `Pawn.bUseControllerRotationPitch` false _returnvalue)
    (`self.SetIgnoreLookInput` false)
    (`self.CheckAndSetMesh`)))

(event `Key|LeftControl`
  (params (Key :type "Key Structure" :default "AnyKey"))
  (bind _returnvalue (`self.K2_GetPawn`))
  ;[0.065 1 0.1309] Setting different presets on the camera. If a preset has not been found, nothing is changed (view stays as is)
  (:`Pressed`
    (`/Game/FinalCamera/Blueprints/FinalCameraManager.SetPresetCameraMode` (cast `/Game/FinalCamera/Blueprints/FinalCameraManager` (`self.PlayerCameraManager`) :!pure true) "FirstPerson" true)
    (set `self.CurrentCameraMode` "FirstPerson")
    (set `Pawn.bUseControllerRotationYaw` true _returnvalue)
    (set `Pawn.bUseControllerRotationPitch` true _returnvalue)
    (`self.CheckAndSetMesh`)))

(event `Key|RightControl`
  (params (Key :type "Key Structure" :default "AnyKey"))
  ;[0.065 1 0.1309] Setting different presets on the camera. If a preset has not been found, nothing is changed (view stays as is)
  (:`Pressed`
    (`/Game/FinalCamera/Blueprints/FinalCameraManager.SetPresetCameraMode` (cast `/Game/FinalCamera/Blueprints/FinalCameraManager` (`self.PlayerCameraManager`) :!pure true) "FirstPersonArms" true)
    (set `self.CurrentCameraMode` "FirstPersonArms")
    (set `self.switchToFirstPerson` true)))

(event `SetArmsMesh`
  (bind _mesh (`Character.Mesh` (cast `Character` (`self.K2_GetPawn`) :!pure true)))
  ;[1 0.07237 0.8154] Helper Event for setting the arms-mesh for that first-person-mode
  (`SceneComponent.SetHiddenInGame` _mesh false false)
  (`SkinnedMeshComponent.SetSkinnedAssetAndUpdate` _mesh "/Game/FinalCamera/Character/Mesh/SK_Mannequin_Arms.SK_Mannequin_Arms" true)
  (`SkeletalMeshComponent.SetAnimInstanceClass` _mesh "/Game/FinalCamera/Character/ArmsAnimBlueprint.ArmsAnimBlueprint_C")
  (`SceneComponent.K2_SetRelativeRotation` _mesh (struct) false false))

(event `HideFullMeshAndSetArms`
  ;[1 0.07237 0.8154] Hides the Skeletal Mesh and sets a timer to set the arms-mesh
  (`SceneComponent.SetHiddenInGame` (`Character.Mesh` (cast `Character` (`self.K2_GetPawn`) :!pure true)) true false)
  (`KismetSystemLibrary.K2_SetTimer` null "SetArmsMesh" 0.22) ; delay the swap of the skeletal mesh or else we see the arms only while zooming in. may need a bit tweaking here
)

(event `self.ReceiveTick`
  (params (DeltaSeconds :type "Float (single-precision)"))
  (bind _returnvalue (`self.K2_GetPawn`))
  ;[1 1 1] If switching to First person, we need to make sure that we swap the meshes correctly. If our Camera distance is less than 40, we hide the actual full mesh and then start a timer to swap the mesh to the correct arms mesh
  (if (`self.switchToFirstPerson`)
    (if (< (`PlayerCameraManager.FreeCamDistance` (cast `/Game/FinalCamera/Blueprints/FinalCameraManager` (`self.PlayerCameraManager`) :!pure true)) 40.0)
      (`self.HideFullMeshAndSetArms`)
      ;[1 1 1] Some more useful stuff for First person;  We want the character to rotate with the controller (which is rotated by mouse)
      (set `Pawn.bUseControllerRotationYaw` true _returnvalue)
      (set `Pawn.bUseControllerRotationPitch` true _returnvalue)
      (set `self.switchToFirstPerson` false) ; Last but not least, reset our switch variable
    )))

(event `self.ReceiveBeginPlay`
  ;[1 1 1] Setup initial camera mode with Topdown Preset
  (`/Game/FinalCamera/Blueprints/FinalCameraManager.SetPresetCameraMode` (cast `/Game/FinalCamera/Blueprints/FinalCameraManager` (`self.PlayerCameraManager`) :!pure true) "TopDown" false)
  ;[1 1 1] Tutorial widget stuff
  (bind _returnvalue (`|CreateWidget` "/Game/FinalCamera/Blueprints/UMG/Tutorial.Tutorial_C"))
  (bind _output_get (set `self.HUD Reference` _returnvalue))
  (`UserWidget.AddToViewport` _output_get 0))

(fn `ResetPitch`
  (bind _returnvalue (`KismetMathLibrary.MakeRotator` (.roll (`self.GetControlRotation`)) 0.0 (.yaw (`self.GetControlRotation`))))
  (`self.SetControlRotation` _returnvalue)
  (`self.K2_SetActorRotation` (`self.K2_GetPawn`) _returnvalue false))

(fn `UserConstructionScript`)