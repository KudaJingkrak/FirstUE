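; Player controller for a local multiplayer camera demo that keeps each player's character from leaving the screen.
; Every tick it projects the pawn to screen space and, near a viewport edge, launches the character horizontally toward the players' center.
; GetCenterOfPlayers compares character pairs to find the farthest two and uses their midpoint as that center.
; A separate CheckAndSetMesh graph applies the mannequin mesh, animation Blueprint and rotation.
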(event `self.ReceiveTick`
  (params (DeltaSeconds :type "Float (single-precision)"))
  (bind (_sizex _sizey) (`self.GetViewportSize`))
  (bind (_x _y) (`KismetMathLibrary.BreakVector2D` (`self.ProjectWorldLocationToScreen` (`self.K2_GetActorLocation` (`self.K2_GetPawn`)))))
  ;[1 1 1] If a player gets to the edge of the screen...
  (if (or (<= _x 20.0) (<= _y 20.0) (>= _x (`KismetMathLibrary.Conv_IntToDouble` (- _sizex 20))) (>= _y (`KismetMathLibrary.Conv_IntToDouble` (- _sizey 20))))
    ;[1 1 1] ...find the right direction to the center of the screen...
    (bind _center (`self.GetCenterOfPlayers`))
    ;[1 1 1] ...and push him back there
    (`Character.LaunchCharacter` (cast `Character` (`self.K2_GetPawn`) :!pure true) (* (`KismetMathLibrary.GetForwardVector` (`KismetMathLibrary.FindLookAtRotation` (`self.K2_GetActorLocation` (`self.K2_GetPawn`)) _center)) 500.0) true false)))

(fn `GetCenterOfPlayers`
  (returns (center :type "Vector Structure"))
  (locals (tmpVec :type "Vector Structure") (savedPlayer1 :type "Actor Object Reference") (savedPlayer2 :type "Actor Object Reference") (maxDist :type "Float (double-precision)"))
  (bind _savedplayer1 (`local.savedPlayer1`))
  (bind _savedplayer2 (`local.savedPlayer2`))
  (bind _returnvalue (`GameModeBase.GetNumPlayers` (`GameplayStatics.GetGameMode`)))
  (bind _returnvalue_2 (- _returnvalue 1))
  (for _index (range (+ _returnvalue_2 1))
    (for _index_2 (range (+ _returnvalue_2 1))
      (if (not (== _index_2 _index))
        (bind _returnvalue_3 (`GameplayStatics.GetPlayerCharacter` _index))
        (bind _returnvalue_4 (`GameplayStatics.GetPlayerCharacter` _index_2))
        (bind _returnvalue_5 (`KismetMathLibrary.VSize` (- (`self.K2_GetActorLocation` _returnvalue_3) (`self.K2_GetActorLocation` _returnvalue_4))))
        (if (> _returnvalue_5 (`local.maxDist`))
          (set `local.maxDist` _returnvalue_5)
          (set `local.savedPlayer1` _returnvalue_3)
          (set `local.savedPlayer2` _returnvalue_4))))
    (return (`local.tmpVec`)))
  (`/Engine/EditorBlueprintResources/StandardMacros.IsValid` _savedplayer1
    (:`Is Valid`
      (`/Engine/EditorBlueprintResources/StandardMacros.IsValid` _savedplayer2
        (:`Is Valid`
          (set `local.tmpVec` (/ (+ (`self.K2_GetActorLocation` _savedplayer1) (`self.K2_GetActorLocation` _savedplayer2)) 2.0)))
        (:`Is Not Valid`
          _)))
    (:`Is Not Valid`
      _))
  (return (`local.tmpVec`)))

(fn `UserConstructionScript`)