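; RTSGamePC is a sample player controller that drives the FinalCameraManager for an RTS-style camera, applying its "RTS" preset on BeginPlay.
; It forwards scrolling-mode toggle, zoom, free look and mouse axis inputs to the camera manager.
; Releasing Select traces the Camera channel under the cursor and makes the hit actor the camera target, while DeSelect clears the target and unlocks position.
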(event `InputAction|EnableDisableScrollingMode`
  (params (Key :type "Key Structure" :default "AnyKey"))
  ;[0.03787 1 0.1633] Forward Inputs to camera
  ;;[1 1 1] Switches Scrolling mode on and off
  (:`Pressed`
    (`/Game/FinalCamera/Blueprints/FinalCameraManager.SwitchScrollingModeOnOff` (cast `/Game/FinalCamera/Blueprints/FinalCameraManager` (`self.PlayerCameraManager`) :!pure true))))

(event `InputAction|ZoomIn`
  (params (Key :type "Key Structure" :default "AnyKey"))
  ;[0.03787 1 0.1633] Forward Inputs to camera
  ;;[1 1 1] ZoomIn and ZoomOut; i guess this explains itself?
  (:`Pressed`
    (`/Game/FinalCamera/Blueprints/FinalCameraManager.ZoomInEvent` (cast `/Game/FinalCamera/Blueprints/FinalCameraManager` (`self.PlayerCameraManager`) :!pure true))))

(event `InputAction|ZoomOut`
  (params (Key :type "Key Structure" :default "AnyKey"))
  ;[0.03787 1 0.1633] Forward Inputs to camera
  ;;[1 1 1] ZoomIn and ZoomOut; i guess this explains itself?
  (:`Pressed`
    (`/Game/FinalCamera/Blueprints/FinalCameraManager.ZoomOutEvent` (cast `/Game/FinalCamera/Blueprints/FinalCameraManager` (`self.PlayerCameraManager`) :!pure true))))

(event `InputAction|FreeLook`
  (params (Key :type "Key Structure" :default "AnyKey"))
  ;[0.03787 1 0.1633] Forward Inputs to camera
  (:`Pressed`
    (`/Game/FinalCamera/Blueprints/FinalCameraManager.FreeCamModeEventOn` (cast `/Game/FinalCamera/Blueprints/FinalCameraManager` (`self.PlayerCameraManager`) :!pure true)) ; FreeCamMode On means, no snapback to any original location
  ))

(event `InputAxis|aMouseX` :consume false
  (params (AxisValue :type "Float (single-precision)"))
  ;[0.03787 1 0.1633] Forward Inputs to camera
  ;;[1 1 1] Forward mouse axis values to the CameraManager
  (`/Game/FinalCamera/Blueprints/FinalCameraManager.RawMouseEvent` (cast `/Game/FinalCamera/Blueprints/FinalCameraManager` (`self.PlayerCameraManager`) :!pure true) AxisValue (stale `InputAxis|aMouseY` AxisValue) :!label _label))

(event `InputAxis|aMouseY` :consume false
  (params (AxisValue :type "Float (single-precision)"))
  ;[0.03787 1 0.1633] Forward Inputs to camera
  ;;[1 1 1] Forward mouse axis values to the CameraManager
  (goto _label))

(event `InputAction|DeSelect`
  (params (Key :type "Key Structure" :default "AnyKey"))
  (bind _asfinal_camera_manager (cast `/Game/FinalCamera/Blueprints/FinalCameraManager` (`self.PlayerCameraManager`) :!pure true))
  ;[1 0.9793 0.0173] Reset our current Camera Target
  (:`Pressed`
    (`/Game/FinalCamera/Blueprints/FinalCameraManager.SetTargetActor` _asfinal_camera_manager null)
    (set `/Game/FinalCamera/Blueprints/FinalCameraManager.lockPosition` false _asfinal_camera_manager)))

(event `InputAction|Select`
  (params (Key :type "Key Structure" :default "AnyKey"))
  (bind (_bblockinghit _binitialoverlap _time _location _impactpoint _normal _impactnormal _physmat _hitactor) (`GameplayStatics.BreakHitResult` (`self.GetHitResultUnderCursorByChannel` "TraceTypeQuery2" true)))
  ;[1 0.9793 0.0173] If we clicked anywhere, set our new cameratarget to the actor we clicked on
  (:`Released`
    (if _bblockinghit
      (`/Engine/EditorBlueprintResources/StandardMacros.IsValid` _hitactor
        (:`Is Valid`
          (`/Game/FinalCamera/Blueprints/FinalCameraManager.SetTargetActor` (cast `/Game/FinalCamera/Blueprints/FinalCameraManager` (`self.PlayerCameraManager`) :!pure true) _hitactor))))))

(event `self.ReceiveBeginPlay`
  ;[0.08737 0.1594 1] Setup initial camera mode with RTS Preset
  (`/Game/FinalCamera/Blueprints/FinalCameraManager.SetPresetCameraMode` (cast `/Game/FinalCamera/Blueprints/FinalCameraManager` (`self.PlayerCameraManager`) :!pure true) "RTS" false))

(event `self.ReceiveTick`
  (params (DeltaSeconds :type "Float (single-precision)")))

(fn `UserConstructionScript`)