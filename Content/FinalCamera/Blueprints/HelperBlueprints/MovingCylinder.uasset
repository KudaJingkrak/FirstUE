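; MovingCylinder is an actor that travels through BP_Waypoint actors in Sequence order, intended to loop back to the first.
; BeginPlay targets waypoint 0, and overlapping any waypoint targets the next sequence number, or 0 if that lookup is invalid.
; Tick faces the target and steps toward it by a fixed distance per frame, without delta-time scaling or sweep.
; GetWayPointBySeq finds waypoints by scanning all BP_Waypoint actors on each call.
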(event EventBeginPlay
  (bind _foundwaypoint (CallFunction|GetWayPointbySeq))
  (Variables|Default|SettargetLoc (Transformation|GetActorLocation _foundwaypoint)))

(event Collision|EventActorBeginOverlap
  (params (OtherActor :type Actor%20Object%20Reference))
  (bind _asbp_waypoint (Utilities|Casting|CastToBP_Waypoint OtherActor))
  (bind _foundwaypoint (CallFunction|GetWayPointbySeq (+ (Variables|/Game/FinalCamera/Blueprints/HelperBlueprints/BP_Waypoint.BP_Waypoint_C|Getsequence _asbp_waypoint) 1)))
  (Utilities|IsValid _foundwaypoint
    (:Is%20Valid
      (Variables|Default|SettargetLoc (Transformation|GetActorLocation _foundwaypoint)))
    (:Is%20Not%20Valid
      (bind _foundwaypoint_2 (CallFunction|GetWayPointbySeq))
      (Variables|Default|SettargetLoc (Transformation|GetActorLocation _foundwaypoint_2)))))

(event EventTick
  (params (DeltaSeconds :type Float%20%28single-precision%29))
  (bind _returnvalue (Transformation|GetActorLocation))
  (bind _targetloc (Variables|Default|GettargetLoc))
  (bind _returnvalue_2 (Math|Rotator|FindLookatRotation _returnvalue _targetloc))
  (Transformation|SetActorRotation _returnvalue_2)
  (Transformation|SetActorLocation (+ (Transformation|GetActorLocation) (* (Math|Vector|GetForwardVector _returnvalue_2) 2.0)) false))

(fn ConstructionScript)

(fn GetWayPointbySeq
  (params (seq :type Integer))
  (bind _outactors (Actor|GetAllActorsOfClass "/Game/FinalCamera/Blueprints/HelperBlueprints/BP_Waypoint.BP_Waypoint_C"))
  (bind _array_element (Utilities|Array|ForEachLoopwithBreak _outactors :!label _label)
    (:LoopBody
      (if (== (Variables|/Game/FinalCamera/Blueprints/HelperBlueprints/BP_Waypoint.BP_Waypoint_C|Getsequence _array_element) seq)
        (LocalVariables|SetcurrentWayPoint _array_element)
        (goto _label Break)))
    (:Completed
      (return (LocalVariables|GetcurrentWayPoint)))))