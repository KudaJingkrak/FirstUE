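; Pickup actor that sends a pickup message when the player pawn overlaps it, then hides and expires shortly after.
; A looping one-second timer checks player distance and, within range, line-traces from the player until a PickupActor hit marks it discovered.
; Once discovered, nearby pickups toggle custom depth on their mesh based on whether its location projects to screen, clearing it when out of range.
; The trace leaves debug drawing enabled.
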(event `self.ReceiveBeginPlay`
  (`KismetSystemLibrary.K2_SetTimer` null "CheckPlayerLookedMe" 1.0 true))

(event `self.ReceiveActorBeginOverlap`
  (params (OtherActor :type "Actor Object Reference"))
  (if (== OtherActor (`GameplayStatics.GetPlayerPawn` 0))
    (message `/Game/Blueprints/Interfaces/Usable.Pickup` (`self.Pickup`) OtherActor)
    (`self.SetActorHiddenInGame` true)
    (`self.SetLifeSpan` 0.3)))

(fn `CheckPlayerLookedMe`
  (if (> (`self.PlayerDistance`) 500.0)
    (`PrimitiveComponent.SetRenderCustomDepth` (`self.PickupMesh`) false)
    (elif (not (`self.isDiscovered`))
      (bind _outhit (`KismetSystemLibrary.LineTraceSingle` :`Start` (`self.K2_GetActorLocation` (`GameplayStatics.GetPlayerPawn` 0)) :`End` (`SceneComponent.K2_GetComponentLocation` (`self.PickupMesh`)) :`TraceChannel` "TraceTypeQuery1" :`DrawDebugType` "ForDuration" :`bIgnoreSelf` false))
      (cast `/Game/Blueprints/PickupActor` (`.HitActor` (`GameplayStatics.BreakHitResult` _outhit)))
      (set `self.isDiscovered` true)
      (else
        (`PrimitiveComponent.SetRenderCustomDepth` (`self.PickupMesh`) (`.ReturnValue` (`PlayerController.ProjectWorldLocationToScreen` (`GameplayStatics.GetPlayerController` 0) (`SceneComponent.K2_GetComponentLocation` (`self.PickupMesh`)) false)))))))

(fn `UserConstructionScript`)