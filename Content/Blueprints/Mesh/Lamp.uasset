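; Lamp actor with a spotlight and a cone overlap volume that marks when player-controlled characters are inside its light.
; Entering the cone turns off custom depth rendering on the actor's skeletal mesh and leaving turns it back on, skipping AI and actors without an instigator controller.
; The construction script derives the spotlight's attenuation radius and outer cone angle from the cone's world scale.
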(event `self.Cone.OnComponentBeginOverlap`
  (params (OverlappedComponent :type "PrimitiveComponent Object Reference") (OtherActor :type "Actor Object Reference") (OtherComp :type "PrimitiveComponent Object Reference") (OtherBodyIndex :type Integer) (bFromSweep :type Boolean) (SweepResult :type "HitResult Structure (by ref)"))
  (bind _returnvalue (`self.GetComponentByClass` OtherActor "/Script/Engine.SkeletalMeshComponent"))
  ;[1 1 1] Not AI
  (`/Engine/EditorBlueprintResources/StandardMacros.IsValid` (`AIBlueprintHelperLibrary.GetAIController` OtherActor)
    (:`Is Not Valid`
      ;[1 1 1] Has Controller
      (`/Engine/EditorBlueprintResources/StandardMacros.IsValid` (`self.GetInstigatorController` OtherActor)
        (:`Is Valid`
          (`/Engine/EditorBlueprintResources/StandardMacros.IsValid` _returnvalue
            (:`Is Valid`
              (`PrimitiveComponent.SetRenderCustomDepth` _returnvalue false))))))))

(event `self.Cone.OnComponentEndOverlap`
  (params (OverlappedComponent :type "PrimitiveComponent Object Reference") (OtherActor :type "Actor Object Reference") (OtherComp :type "PrimitiveComponent Object Reference") (OtherBodyIndex :type Integer))
  (bind _returnvalue (`self.GetComponentByClass` OtherActor "/Script/Engine.SkeletalMeshComponent"))
  ;[1 1 1] Not AI
  (`/Engine/EditorBlueprintResources/StandardMacros.IsValid` (`AIBlueprintHelperLibrary.GetAIController` OtherActor)
    (:`Is Not Valid`
      ;[1 1 1] Has Controller
      (`/Engine/EditorBlueprintResources/StandardMacros.IsValid` (`self.GetInstigatorController` OtherActor)
        (:`Is Valid`
          (`/Engine/EditorBlueprintResources/StandardMacros.IsValid` _returnvalue
            (:`Is Valid`
              (`PrimitiveComponent.SetRenderCustomDepth` _returnvalue true))))))))

(fn `UserConstructionScript`
  (bind _spotlight (`self.SpotLight`))
  (bind _returnvalue (`SceneComponent.K2_GetComponentToWorld` (`self.Cone`)))
  (bind _returnvalue_2 (* (.z (.scale _returnvalue)) 100.0))
  (bind _returnvalue_3 (* (`KismetMathLibrary.FMax` (.x (.scale _returnvalue)) (.y (.scale _returnvalue))) 50.0))
  (`LocalLightComponent.SetAttenuationRadius` _spotlight (* (`KismetMathLibrary.Sqrt` (+ (`KismetMathLibrary.MultiplyMultiply_FloatFloat` _returnvalue_3 2.0) (`KismetMathLibrary.MultiplyMultiply_FloatFloat` _returnvalue_2 2.0))) 1.5))
  (`SpotLightComponent.SetOuterConeAngle` _spotlight (/ (`KismetMathLibrary.DegAtan` (/ _returnvalue_2 _returnvalue_3)) 2.0)))