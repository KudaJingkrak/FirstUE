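; BP_Ground is a procedural ground actor that lays out a flat grid of static mesh tiles sized by X, Y and Size.
; The construction script builds it with nested loops, with no active event logic.
; With UseDecal on, about one tile in ten gets a small scatter of extra static meshes, split 70/30 between two add-component branches.
; Scatter is randomly offset around tile origins and unseeded, so it changes whenever construction reruns.
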(fn `UserConstructionScript`
  (bind (_returnvalue_x _returnvalue_y) (`KismetMathLibrary.BreakVector` (`KismetMathLibrary.RandomUnitVector`)))
  (bind _size (`self.size`))
  (for _index (range (+ (`self.X`) 1))
    (for _index_2 (range (+ (`self.Y`) 1))
      (bind _returnvalue (`KismetMathLibrary.MakeVector` (* _index _size) (* _index_2 _size)))
      (`AddComponent|NODE_AddStaticMeshComponent-1` :`RelativeTransform` (`KismetMathLibrary.MakeTransform` _returnvalue))
      (if (and (`self.useDecal`) (>= (`KismetMathLibrary.RandomFloat`) 0.9))
        (for _ (range (+ (`KismetMathLibrary.RandomInteger` 5) 1))
          (if (>= (`KismetMathLibrary.RandomFloat`) 0.3)
            (bind _returnvalue_2 (`KismetMathLibrary.MakeTransform` (+ _returnvalue (* (`KismetMathLibrary.MakeVector` _returnvalue_x _returnvalue_y) (`KismetMathLibrary.RandomFloatInRange` 0.0 (* (`self.size`) 0.33333))))))
            (`AddComponent|NODE_AddStaticMeshComponent-4` :`RelativeTransform` _returnvalue_2)
            (else
              (`AddComponent|NODE_AddStaticMeshComponent-5` :`RelativeTransform` _returnvalue_2))))))))