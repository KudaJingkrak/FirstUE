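; Light path actor that lines a spline with pairs of rect lights at construction time.
; The construction script loops over spline points, passing each point's location plus tangent, and its rotation, to SpawnPathLight.
; That function adds two lights offset half the path size along local Y, yawed in opposite directions, with shared color, intensity and attenuation radius.
; GetSplinePointData holds only unconnected spline getters, and a leftover debug print runs per point.
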(fn `SpawnPathLight`
  (params (MaualAttachment :type Boolean) (RelativeTransform :type "Transform Structure") (PathSize :type "Float (double-precision)"))
  (bind _location (.location RelativeTransform))
  (bind _rotation (.rotation RelativeTransform))
  (bind _returnvalue (* PathSize 0.5))
  (bind _lightcolor (`self.LightColor`))
  (bind _intesity (`self.Intesity`))
  (bind _attenuationradius (`self.AttenuationRadius`))
  (`|ExecutionSequence`
    (:`then_0`
      (bind _returnvalue_2 (`AddComponent|NODE_AddRectLightComponent-3` :`bManualAttachment` MaualAttachment :`RelativeTransform` (`KismetMathLibrary.MakeTransform` (- _location (`KismetMathLibrary.MakeVector` 0.0 _returnvalue)) _rotation)))
      (`LocalLightComponent.SetAttenuationRadius` _returnvalue_2 _attenuationradius)
      (`LightComponent.SetLightColor` _returnvalue_2 _lightcolor true)
      (`LightComponent.SetIntensity` _returnvalue_2 _intesity)
      (`SceneComponent.K2_AddRelativeRotation` _returnvalue_2 (struct :`Yaw` 90.0) false false))
    (:`then_1`
      (bind _returnvalue_3 (`AddComponent|NODE_AddRectLightComponent-4` :`bManualAttachment` MaualAttachment :`RelativeTransform` (`KismetMathLibrary.MakeTransform` (+ _location (`KismetMathLibrary.MakeVector` 0.0 _returnvalue)) _rotation)))
      (`LocalLightComponent.SetAttenuationRadius` _returnvalue_3 _attenuationradius)
      (`LightComponent.SetLightColor` _returnvalue_3 _lightcolor true)
      (`LightComponent.SetIntensity` _returnvalue_3 _intesity)
      (`SceneComponent.K2_AddRelativeRotation` _returnvalue_3 (struct :`Yaw` -90.0) false false))))

(fn `UserConstructionScript`
  (for _index (range (`SplineComponent.GetNumberOfSplinePoints` (`self.Spline`)))
    (`KismetSystemLibrary.PrintString` (`KismetStringLibrary.Conv_VectorToString` (0.0 0.0 0.0)))
    (bind (_location _tangent _rotation) (`self.GetSplinePointData` _index))
    (`self.SpawnPathLight` false (`KismetMathLibrary.MakeTransform` (+ _location _tangent) _rotation) (`self.PathSize`))))