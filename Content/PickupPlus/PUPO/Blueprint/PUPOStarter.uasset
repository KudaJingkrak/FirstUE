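; PUPOStarter detects objects the player can pick up or inspect and gates input to the PUPOMain actor accordingly.
; On BeginPlay it copies limits from MainSettings and spawns PUPOMain if none exists, storing only that spawned reference.
; Each Tick, unless pickup is pressed or active, it traces from the camera.
; Light enough physics objects (when allowed) or components tagged PUPOInspect enable PUPOMain's input; otherwise DeactivatePUPO disables it.
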(event `self.ReceiveBeginPlay`
  (bind (_mainsettings_maxgrabdistance _mainsettings_maxcarryweight _mainsettings_canpickupphysicsobjects) (break `/Game/PUPO/Blueprint/PUPOMainSettings` (`self.MainSettings`)))
  (`self.EnableInput` (`GameplayStatics.GetPlayerController` (`self.PlayerIndex`)))
  (set `self.MaxGrabDistance` _mainsettings_maxgrabdistance)
  (set `self.MaxCarryHeight` _mainsettings_maxcarryweight)
  (set `self.CanPickUpPhysicsObjects` _mainsettings_canpickupphysicsobjects)
  ;[1 1 1] Spawn PUPOMain if there is no any
  (bind _outactors (`GameplayStatics.GetAllActorsOfClass` "/Game/PUPO/Blueprint/Misc/PUPOMain.PUPOMain_C"))
  (if (== (`KismetArrayLibrary.Array_Length` _outactors) 0)
    (bind _returnvalue (`|SpawnActorFromClass` "/Game/PUPO/Blueprint/Misc/PUPOMain.PUPOMain_C" (`KismetMathLibrary.MakeTransform` (0.0 0.0 0.0)) "AlwaysSpawn" "OverrideRootScale")) ; Spawn PUPO BP Actor to be able to pick up.
    (set `self.PUPOMain` _returnvalue)))

(event `self.ReceiveTick`
  (params (DeltaSeconds :type "Float (single-precision)"))
  (bind _playerindex (`self.PlayerIndex`))
  (bind _returnvalue (`GameplayStatics.GetPlayerCameraManager` _playerindex))
  (bind _returnvalue_2 (`PlayerCameraManager.GetCameraLocation` _returnvalue))
  (if (not (or (`self.[PUPO]PickUpPressed`) (`self.PUPOActive`)))
    (bind _outhit (`KismetSystemLibrary.LineTraceSingle` _returnvalue_2 (+ _returnvalue_2 (* (`self.GetActorForwardVector` _returnvalue) (`self.MaxGrabDistance`))) "TraceTypeQuery1" false (`|MakeArray` (`GameplayStatics.GetPlayerPawn` _playerindex) :!type "Actor Object Reference") "ForOneFrame"))
    (if (`GameplayStatics.BreakHitResult` _outhit)
      (`/Engine/EditorBlueprintResources/StandardMacros.IsValid` (`.HitActor` (`GameplayStatics.BreakHitResult` _outhit))
        (:`Is Valid`
          (bind _output_get (set `self.HitComponent` (`.HitComponent` (`GameplayStatics.BreakHitResult` _outhit))))
          (`/Engine/EditorBlueprintResources/StandardMacros.IsValid` _output_get
            (:`Is Valid`
              (set `self.HitLocation` (`.Location` (`GameplayStatics.BreakHitResult` _outhit)))
              (`/Engine/EditorBlueprintResources/StandardMacros.IsValid` (`self.PUPOMain`)
                (:`Is Valid`
                  (if (and (`SceneComponent.IsAnySimulatingPhysics` (`self.HitComponent`)) (`self.CanPickUpPhysicsObjects`))
                    (if (< (`PrimitiveComponent.GetMass` (`self.HitComponent`)) (`self.MaxCarryHeight`))
                      (`self.EnableInput` (`self.PUPOMain`) (`GameplayStatics.GetPlayerController` (`self.PlayerIndex`)) :!label _label)
                      (else
                        (`self.DeactivatePUPO` :!label _label_2)))
                    (else
                      (bind _output_get_2 (set `self.PUPOInspect` (`ActorComponent.ComponentHasTag` (`self.HitComponent`) "PUPOInspect")))
                      (if _output_get_2
                        (goto _label)
                        (else
                          (goto _label_2))))))
                (:`Is Not Valid`
                  (goto _label_2))))
            (:`Is Not Valid`
              (`self.DeactivatePUPO` :!label _label_3))))
        (:`Is Not Valid`
          (goto _label_3)))
      (else
        (goto _label_3)))))

(event `InputAction|[PUPO]Pick Up/Inspect` :consume false
  (params (Key :type "Key Structure" :default "AnyKey"))
  (:`Pressed`
    (set `self.[PUPO]PickUpPressed` true))
  (:`Released`
    (set `self.[PUPO]PickUpPressed` false)))

(event `DeactivatePUPO`
  (bind _pupomain (`self.PUPOMain`))
  (`/Engine/EditorBlueprintResources/StandardMacros.IsValid` _pupomain
    (:`Is Valid`
      (`self.DisableInput` _pupomain (`GameplayStatics.GetPlayerController` (`self.PlayerIndex`)))
      (set `self.PUPOActive` false)
      (set `self.PUPOInspect` false))))

(fn `UserConstructionScript`)